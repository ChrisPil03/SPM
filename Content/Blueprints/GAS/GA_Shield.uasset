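; GA_Shield is a Gameplay Ability that gives the player a timed shield with an on-screen indicator.
; On activation it casts the avatar to PlayerCharacter, applies GE_DamageReduction through ApplyGameplayEffectToTarget, shows WBP_Shield, and ends itself after a fixed delay.
; The widget is created on first use, cached for reuse, and hidden when the ability ends.
; Debug prints mark each stage, and a failed cast stops activation without calling EndAbility.
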(event `self.K2_ActivateAbility`
  (`KismetSystemLibrary.PrintString` "Hello")
  (cast `PlayerCharacter` (`self.GetAvatarActorFromActorInfo`))
  (`KismetSystemLibrary.PrintString` "Apply GE")
  (`self.BP_ApplyGameplayEffectToTarget` (struct) "/Game/Blueprints/GAS/GE_DamageReduction.GE_DamageReduction_C")
  (`self.ShowShieldUI`)
  (`AbilityTask_WaitDelay.WaitDelay` 5.0
    (:`OnFinish`
      (`self.K2_EndAbility`))))

(event `self.K2_OnEndAbility`
  (params (bWasCancelled :type Boolean))
  (`KismetSystemLibrary.PrintString` "Ended")
  (`self.HideShieldUI`))

(event `ShowShieldUI`
  (bind _shieldwidgetref (`self.ShieldWidgetRef`)
    (:`then`
      (`Widget.SetVisibility` _shieldwidgetref "Visible"))
    (:`else`
      (bind _returnvalue (`|CreateWidget` "/Game/Blueprints/Widgets/WBP_Shield.WBP_Shield_C"))
      (bind _output_get (set `self.ShieldWidgetRef` _returnvalue))
      (`UserWidget.AddToViewport` _output_get 0))))

(event `HideShieldUI`
  (bind _shieldwidgetref (`self.ShieldWidgetRef`)
    (:`then`
      (set `Widget.Visibility` "Hidden" _shieldwidgetref))
    (:`else`)))