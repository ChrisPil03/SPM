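; Gameplay ability that makes the GloOrb exploding enemy blow up, damaging nearby actors and destroying itself.
; On activation it commits, casts the owner to BP_ExplodingEnemyAI and runs a sphere overlap around its bounds origin, ignoring itself and drawing a debug sphere.
; It applies the enemy's explosion damage effect to overlapped actors and its self-destruct effect to the owner, then ends.
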(event `self.K2_ActivateAbility`
  (bind _origin (`Actor.GetActorBounds` (`self.Enemy`) false false))
  (`self.K2_CommitAbility`)
  (bind _asbp_exploding_enemy_ai (cast `/Game/Blueprints/AI/BP_ExplodingEnemyAI` (`self.GetOwningActorFromActorInfo`)))
  (set `self.Enemy` _asbp_exploding_enemy_ai)
  (`KismetSystemLibrary.DrawDebugSphere` _origin 300.0)
  (`KismetArrayLibrary.Array_Add` (`self.IgnoreSelf`) (`self.Enemy`))
  (bind _outactors (`KismetSystemLibrary.SphereOverlapActors` _origin 300.0 (`self.ObjectTypes`) null (`self.IgnoreSelf`)))
  (`self.BP_ApplyGameplayEffectToTarget` (`AbilitySystemBlueprintLibrary.AbilityTargetDataFromActorArray` _outactors) (`/Game/Blueprints/AI/BP_ExplodingEnemyAI.ExplosionDamageEffect` (`self.Enemy`)))
  (`self.BP_ApplyGameplayEffectToOwner` (`/Game/Blueprints/AI/BP_ExplodingEnemyAI.SelfDestructEffect` (`self.Enemy`)))
  (`self.K2_EndAbility`))