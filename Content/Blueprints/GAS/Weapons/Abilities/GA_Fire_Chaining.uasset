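; Gameplay Ability for a chaining weapon shot that hits every actor in the received target data.
; ActivateAbility calls the parent and commits; OnTargetDataReady draws debug lines from the BP_Weapon avatar's muzzle to the first target, then between successive targets' bounds centers.
; Each target receives the GEDamage effect before the ability prints a debug string and ends.
; A WaitDelay task is created per later link, but its Finish output drives nothing.
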(event `self.K2_ActivateAbility`
  (`parent.K2_ActivateAbility`)
  (`self.K2_CommitAbility`))

(event `self.OnTargetDataReady`
  (params (TargetData :type "GameplayAbilityTargetDataHandle Structure (by ref)"))
  (bind _returnvalue (`AbilitySystemBlueprintLibrary.GetAllActorsFromTargetData` TargetData))
  (for (_array_element _array_index) _returnvalue
    (bind _output_get (set `self.CurrentEnemyIndex` _array_index))
    (if (== _output_get 0)
      (bind _asbp_weapon (cast `/Game/Blueprints/Weapons/BP_Weapon` (`self.GetAvatarActorFromActorInfo`)))
      (bind _origin (`Actor.GetActorBounds` (`|GetArrayItem` _returnvalue _array_index) false false))
      (`KismetSystemLibrary.DrawDebugLine` (`SceneComponent.K2_GetComponentLocation` (`GunBase.MuzzlePosition` _asbp_weapon)) _origin (struct :`R` 1.0 :`B` 0.53269 :`A` 1.0) 2.0 10.0)
      (else
        (`AbilityTask_WaitDelay.WaitDelay` 0.2
          (:`then`
            _)
          (:`OnFinish`
            _))
        (`KismetSystemLibrary.DrawDebugLine` _origin (`Actor.GetActorBounds` (`|GetArrayItem` _returnvalue (- _array_index 1)) false false) (struct :`R` 1.0 :`B` 0.53269 :`A` 1.0) 2.0 10.0)))
    (`self.BP_ApplyGameplayEffectToTarget` (`AbilitySystemBlueprintLibrary.AbilityTargetDataFromActor` _array_element) (`self.GE Damage`)))
  (`KismetSystemLibrary.PrintString` "Hello")
  (`self.K2_EndAbility`))