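; BP_DownloadZone is a visual effect Blueprint that shows a download zone as a pulsing ring material on a cylinder mesh.
; On BeginPlay it creates a dynamic material instance from MaterialToSet, initializes its ring size and pulse speed, and applies it to the cylinder.
; UpdateRingSize sets the ring size from the supplied value and flips the sign of the pulse speed according to whether the ring is growing.
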(event `self.ReceiveBeginPlay`
  (bind _returnvalue (`KismetMaterialLibrary.CreateDynamicMaterialInstance` (`self.MaterialToSet`)))
  (bind _output_get (set `self.DownloadZoneInstance` _returnvalue))
  (`MaterialInstanceDynamic.SetScalarParameterValue` _output_get "Pulse Speed" 1.0)
  (`MaterialInstanceDynamic.SetScalarParameterValue` _output_get "Ring Size" 0.0)
  (`PrimitiveComponent.SetMaterial` (`self.Cylinder`) 0 _output_get))

(fn `UpdateRingSize`
  (params (Size :type "Float (double-precision)") (IsGrowing :type Boolean))
  (`MaterialInstanceDynamic.SetScalarParameterValue` (`self.DownloadZoneInstance`) "Ring Size" Size)
  (if IsGrowing
    (`MaterialInstanceDynamic.SetScalarParameterValue` (`self.DownloadZoneInstance`) "Pulse Speed" 1.0)
    (else
      (`MaterialInstanceDynamic.SetScalarParameterValue` (`self.DownloadZoneInstance`) "Pulse Speed" -1.0))))

(fn `UserConstructionScript`)