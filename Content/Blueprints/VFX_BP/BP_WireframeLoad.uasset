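; Wireframe load effect actor that animates a level reveal and its reverse on game over through a Material Parameter Collection.
; LoadWireframe staggers timelines driving radius and thickness parameters, then fades the HUD and zeroes a post-process material's weight.
; Game over restores that material, reverses the timelines, shows results, starts menu music and pushes a sound mix.
; O and M keys reset and replay the effect; several per-radius timelines are unwired.
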(event `StartWireframe`
  (bind _zero (`self.Zero`))
  ; Set all values to 0
  (`KismetMaterialLibrary.SetScalarParameterValue` (`self.MPC`) (`self.Thickness`) _zero :!label _label)
  (`KismetMaterialLibrary.SetScalarParameterValue` (`self.MPC`) (`self.FinalThickness`) _zero)
  (`KismetMaterialLibrary.SetScalarParameterValue` (`self.MPC`) (`self.First Radius`) _zero)
  (`KismetMaterialLibrary.SetScalarParameterValue` (`self.MPC`) (`self.Second Radius`) _zero)
  (`KismetMaterialLibrary.SetScalarParameterValue` (`self.MPC`) (`self.Third Radius`) _zero)
  (`KismetMaterialLibrary.SetScalarParameterValue` (`self.MPC`) (`self.Fourth Radius`) _zero)
  (`KismetMaterialLibrary.SetScalarParameterValue` (`self.MPC`) (`self.Fifth Radius`) _zero))

(event `self.ReceiveBeginPlay`
  (`GameplayStatics.PopSoundMixModifier` (`self.SoundMix`))
  (bind _asbp_dive_game_mode (cast `/Game/Blueprints/BP_DiveGameMode` (`GameplayStatics.GetGameMode`)))
  (add `DiveGameMode.OnGameOver` _asbp_dive_game_mode (delegate `OnGameOver_Event`))
  (`self.EnableInput` (`GameplayStatics.GetPlayerController` 0))
  (goto _label))

(event `Key|O`
  (params (Key :type "Key Structure"))
  (:`Pressed`
    (goto _label)))

(event `Key|M`
  (params (Key :type "Key Structure"))
  (:`Pressed`
    (`|ExecutionSequence` :!label _label_2
      (:`then_0`
        (bind (_direction _thickness_track _radius_track) (`Timeline|Timeline` :!via `PlayFromStart` :!label _label_3)
          (:`Update`
            (`KismetMaterialLibrary.SetScalarParameterValue` (`self.MPC`) (`self.First Radius`) _radius_track)
            (`KismetMaterialLibrary.SetScalarParameterValue` (`self.MPC`) (`self.Thickness`) _thickness_track))))
      (:`then_1`
        (`KismetSystemLibrary.Delay` 0.4)
        (bind (_direction_2 _radius_track_2) (`Timeline|Timeline_0` :!via `PlayFromStart` :!label _label_4)
          (:`Update`
            (`KismetMaterialLibrary.SetScalarParameterValue` (`self.MPC`) (`self.Second Radius`) _radius_track_2))))
      (:`then_2`
        (`KismetSystemLibrary.Delay` 1.5)
        (bind (_direction_3 _thickness_track_2 _radius_track_3) (`Timeline|Timeline_3` :!via `PlayFromStart` :!label _label_5)
          (:`Update`
            (`KismetMaterialLibrary.SetScalarParameterValue` (`self.MPC`) (`self.Fifth Radius`) _radius_track_3)
            (`KismetMaterialLibrary.SetScalarParameterValue` (`self.MPC`) (`self.FinalThickness`) _thickness_track_2))))
      (:`then_3`
        (`KismetSystemLibrary.Delay` 2.5)
        (bind _ascyber_warrior_player_controller (cast `CyberWarriorPlayerController` (`GameplayStatics.GetPlayerController` 0)))
        (set `self.As Cyber Warrior Player Controller` _ascyber_warrior_player_controller)
        (bind _aswbp_hud (cast `/Game/Blueprints/Widgets/WBP_HUD` (`CyberWarriorPlayerController.GetHUDWidget` _ascyber_warrior_player_controller)))
        (bind _output_get (set `self.As WBP HUD` _aswbp_hud))
        (`/Game/Blueprints/Widgets/WBP_HUD.PlayFade` _output_get true)
        (`self.SetPostProcessMaterialState` false)))))

(event `LoadWireframe`
  (goto _label_2))

(event `OnGameOver_Event`
  (`/Game/Blueprints/Widgets/WBP_HUD.PlayFade` (`self.As WBP HUD`) false)
  (`self.SetPostProcessMaterialState` true)
  (`|ExecutionSequence`
    (:`then_0`
      (goto _label_5 :!via `ReverseFromEnd`))
    (:`then_1`
      (`KismetSystemLibrary.Delay` 0.4)
      (goto _label_4 :!via `ReverseFromEnd`))
    (:`then_2`
      (`KismetSystemLibrary.Delay` 1.5)
      (goto _label_3 :!via `ReverseFromEnd`))
    (:`then_3`
      (`KismetSystemLibrary.Delay` 5.0)
      (`CyberWarriorPlayerController.DisplayResultScreen` (`self.As Cyber Warrior Player Controller`)))
    (:`then_4`
      (bind _asbp_game_instance (cast `/Game/Blueprints/BP_GameInstance` (`GameplayStatics.GetGameInstance`)))
      (`/Game/Blueprints/BP_GameInstance.PlayMainMenuMusic` _asbp_game_instance))
    (:`then_5`
      (`GameplayStatics.PushSoundMixModifier` (`self.SoundMix`)))))

(event `Key|H`
  (params (Key :type "Key Structure"))
  ; Test Buttons
)

(event `Key|J`
  (params (Key :type "Key Structure"))
  ; Test Buttons
)

(event `Key|K`
  (params (Key :type "Key Structure"))
  ; Test Buttons
)

(event `Key|L`
  (params (Key :type "Key Structure"))
  ; Test Buttons
)

(event `Key|ö`
  (params (Key :type "Key Structure"))
  ; Test Buttons
)

(fn `SetPostProcessMaterialState`
  (params (State :type Boolean))
  (bind _output_get (set `self.LocalSettings` (`PostProcessVolume.Settings` (`self.PostProcessVolume`))))
  (if State
    (bind _weightedblendables_array (break `WeightedBlendables` (break `PostProcessSettings` _output_get)))
    (bind _output (`|GetArrayItem` _weightedblendables_array 1))
    (setmembers `WeightedBlendable` :`StructRef` _output :`Weight` 1.0)
    (else
      (setmembers `WeightedBlendable` :`StructRef` _output :`Weight` 0.0)))
  (set `PostProcessVolume.Settings` (`self.LocalSettings`) (`self.PostProcessVolume`)))

(fn `UserConstructionScript`)