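; BP_Beam is a rifle beam VFX actor with a streaming beam, core sphere and muzzle particles, triggered by StartBeam/EndBeam or the L key.
; Start and end timelines drive sphere scale and MPCRifleBeam material parameters for beam length, mask and sphere glow, alongside Niagara effects.
; Releasing before the StartupTimer threshold reverses the startup timelines; later release plays the fade-out, deactivating muzzle particles and then streaming.
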(event `self.ReceiveBeginPlay`
  ; Set initial values to be sure
  (`self.EnableInput` (`GameplayStatics.GetPlayerController` 0))
  (`SceneComponent.SetWorldScale3D` (`self.SM_CoreSphere`) (0.0 0.0 0.0))
  (`KismetMaterialLibrary.SetScalarParameterValue` (`self.MPC_RifleBeam`) (`self.SphereEmissive`) 1.0)
  (`KismetMaterialLibrary.SetScalarParameterValue` (`self.MPC_RifleBeam`) (`self.SphereExponent`) 1.0))

(event `StartBeam`
  (`|ExecutionSequence` :!label _label
    (:`then_0`
      ; Beam
      (set `self.StartupTimer` 0.0)
      (`ActorComponent.Activate` (`self.NS_Streaming`) false)
      (`KismetMaterialLibrary.SetScalarParameterValue` (`self.MPC_RifleBeam`) (`self.MaskParam`) 1.0)
      (bind (_direction _lengthtrack _timereferencetrack) (`Timeline|BeamStart` :!via `PlayFromStart` :!label _label_2)
        (:`Update`
          (`KismetMaterialLibrary.SetScalarParameterValue` (`self.MPC_RifleBeam`) (`self.LengthParam`) _lengthtrack)
          (set `self.StartupTimer` _timereferencetrack))))
    (:`then_1`
      ; Sphere
      (`SceneComponent.SetWorldScale3D` (`self.SM_CoreSphere`) (0.1 0.1 0.1))
      (`KismetMaterialLibrary.SetScalarParameterValue` (`self.MPC_RifleBeam`) (`self.SphereEmissive`) 1.0)
      (`KismetMaterialLibrary.SetScalarParameterValue` (`self.MPC_RifleBeam`) (`self.SphereExponent`) 1.0)
      (bind (_direction_2 _scaletrack _emissivemult _exponentmult) (`Timeline|SphereStart` :!via `PlayFromStart` :!label _label_3)
        (:`Update`
          (`SceneComponent.SetWorldScale3D` (`self.SM_CoreSphere`) (* _scaletrack (`self.SphereBaseScale`)))
          (`KismetMaterialLibrary.SetScalarParameterValue` (`self.MPC_RifleBeam`) (`self.SphereEmissive`) _emissivemult)
          (`KismetMaterialLibrary.SetScalarParameterValue` (`self.MPC_RifleBeam`) (`self.SphereExponent`) _exponentmult))))
    (:`then_2`
      (`ActorComponent.Activate` (`self.NS_MuzzleParticles`) false)
      (`ActorComponent.Activate` (`self.NS_MuzzleParticlesInitial`) false)
      (`KismetSystemLibrary.Delay` 1.0)
      (`ActorComponent.Deactivate` (`self.NS_MuzzleParticlesInitial`)))
    (:`then_3`
      (`|ExecutionSequence`
        (:`then_0`
          ; Beam
          (bind (_direction_3 _masktrack) (`Timeline|BeamEnd` :!via `Stop` :!label _label_4)
            (:`Update`
              (`KismetMaterialLibrary.SetScalarParameterValue` (`self.MPC_RifleBeam`) (`self.MaskParam`) _masktrack))
            (:`Finished`
              (`ActorComponent.Deactivate` (`self.NS_Streaming`)))))
        (:`then_1`
          ; Sphere
          (bind (_direction_4 _scaletrack_2 _emissivetrack) (`Timeline|SphereEnd` :!via `Stop` :!label _label_5)
            (:`Update`
              (`SceneComponent.SetWorldScale3D` (`self.SM_CoreSphere`) (* _scaletrack_2 (`self.SphereBaseScale`)))
              (`KismetMaterialLibrary.SetScalarParameterValue` (`self.MPC_RifleBeam`) (`self.SphereEmissive`) _emissivetrack))))))))

(event `Key|L`
  (params (Key :type "Key Structure"))
  (:`Pressed`
    (goto _label))
  (:`Released`
    (if (< (`self.StartupTimer`) 0.9) :!label _label_6
      (`|ExecutionSequence`
        (:`then_0`
          (goto _label_2 :!via `Reverse`))
        (:`then_1`
          ; Sphere
          (if (< (`self.StartupTimer`) 0.9)
            (goto _label_3 :!via `Reverse`))))
      (else
        (`|ExecutionSequence`
          (:`then_0`
            (goto _label_2 :!via `Stop`))
          (:`then_1`
            (goto _label_3 :!via `Stop`))
          (:`then_2`
            (`|ExecutionSequence`
              (:`then_0`
                (goto _label_4 :!via `PlayFromStart`))
              (:`then_1`
                (goto _label_5 :!via `PlayFromStart`))
              (:`then_2`
                ; Deactivate
                (`ActorComponent.Deactivate` (`self.NS_MuzzleParticles`))
                (`ActorComponent.Deactivate` (`self.NS_MuzzleParticlesInitial`))))))))))

(event `EndBeam`
  (goto _label_6))

(event `DeactivateAll`
  (`ActorComponent.Deactivate` (`self.NS_Streaming`))
  (`ActorComponent.Deactivate` (`self.NS_MuzzleParticles`))
  (`ActorComponent.Deactivate` (`self.NS_MuzzleParticlesInitial`)))

(fn `NewFunction`)

(fn `UserConstructionScript`)