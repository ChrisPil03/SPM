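; BP_WaspProjectileTESTFIRE is a test actor that fires a Niagara projectile effect when Q is pressed.
; It enables player input on BeginPlay, and FireProjectile spawns the system at the actor's location, stores it and flags it movable.
; Tick slides the stored system along world +Y by Speed and prints the new Y value.
; Only the most recently fired system moves, with no collision or stop logic.
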(event `self.ReceiveBeginPlay`
  (`self.EnableInput` (`GameplayStatics.GetPlayerController` 0)))

(event `Key|Q`
  (params (Key :type "Key Structure"))
  (:`Pressed`
    (`self.FireProjectile`)))

(event `self.ReceiveTick`
  (params (DeltaSeconds :type "Float (single-precision)"))
  (bind _niagarasysteminstance (`self.NiagaraSystemInstance`))
  (bind (_returnvalue_x _returnvalue_y _returnvalue_z) (`KismetMathLibrary.BreakVector` (`SceneComponent.K2_GetComponentLocation` _niagarasysteminstance)))
  (bind _returnvalue (+ _returnvalue_y (* DeltaSeconds (`self.Speed`))))
  (if (`self.IsMovable`)
    (`SceneComponent.K2_SetWorldLocation` _niagarasysteminstance (`KismetMathLibrary.MakeVector` _returnvalue_x _returnvalue _returnvalue_z) false false)
    (`KismetSystemLibrary.PrintString` (`KismetStringLibrary.Conv_DoubleToString` _returnvalue))))

(fn `FireProjectile`
  (locals (NS :type "NiagaraSystem Object Reference" :default "/Script/Niagara.NiagaraSystem'/Game/Assets/Particles/NS_WaspProjectileYellow.NS_WaspProjectileYellow'"))
  (bind _returnvalue (`NiagaraFunctionLibrary.SpawnSystemAtLocation` (`local.NS`) (`self.K2_GetActorLocation`)))
  (set `self.NiagaraSystemInstance` _returnvalue)
  (set `self.IsMovable` true))

(fn `UserConstructionScript`)