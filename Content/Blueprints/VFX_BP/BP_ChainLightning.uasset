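; BP_ChainLightning is a VFX actor that draws a Niagara lightning arc between a Start and an End point.
; BeginPlay places Start at the actor's location and enables player input so the V key can test-fire.
; FireArc moves End to Target, activates the Niagara system and passes End's location as the BeamEnd parameter.
; A note intends weapon or gas triggers to replace the key; a sphere-jitter test timeline is unconnected.
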(event `self.ReceiveBeginPlay`
  (`self.SetStartPosition` (`self.K2_GetActorLocation`))
  (`self.EnableInput` (`GameplayStatics.GetPlayerController` 0)))

(event `Key|V`
  (params (Key :type "Key Structure"))
  ; Instead of this, trigger "Fire Arc At" from weapon/gas and give location of second point for the effect
  (:`Pressed`
    (`self.FireArc`)))

(fn `FireArc`
  (bind _ns_lightningarc (`self.NS_LightningArc`))
  (`SceneComponent.K2_SetWorldLocation` (`self.End`) (`self.Target`) false true)
  (`ActorComponent.Activate` _ns_lightningarc true)
  (`FXSystemComponent.SetVectorParameter` _ns_lightningarc "BeamEnd" (`SceneComponent.K2_GetComponentLocation` (`self.End`))))

(fn `SetStartPosition`
  (params (LocationVector :type "Vector Structure"))
  (`SceneComponent.K2_SetWorldLocation` (`self.Start`) LocationVector false true))

(fn `UserConstructionScript`)