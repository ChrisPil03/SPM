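; Behavior tree service that flags when the AI's target actor has moved far enough to need a new path.
; Each tick, it compares the target's location to the stored previous position using squared distance against a squared movement threshold.
; It writes the result to a recalculation bool on the blackboard, then saves the current location, so movement is measured per tick rather than cumulatively.
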(event `self.ReceiveTickAI`
  (params (OwnerController :type "AIController Object Reference") (ControlledPawn :type "Pawn Object Reference") (DeltaSeconds :type "Float (single-precision)"))
  (bind _movementthreshold (`self.MovementThreshold`))
  (bind _returnvalue (`BTFunctionLibrary.GetBlackboardValueAsActor` (`self.TargetActorKey`)))
  (bind _returnvalue_2 (`Actor.K2_GetActorLocation` _returnvalue))
  (`/Engine/EditorBlueprintResources/StandardMacros.IsValid` _returnvalue
    (:`Is Valid`
      (`BTFunctionLibrary.SetBlackboardValueAsBool` (`self.PathNeedsRecalculationKey`) (>= (`KismetMathLibrary.Vector_DistanceSquared` (`BTFunctionLibrary.GetBlackboardValueAsVector` (`self.PreviousPosition`)) _returnvalue_2) (* _movementthreshold _movementthreshold)))
      (`BTFunctionLibrary.SetBlackboardValueAsVector` (`self.PreviousPosition`) _returnvalue_2))))