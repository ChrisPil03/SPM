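; Behavior tree task that finds a 3D path for a flying enemy to its target using NavigationVolume3D.
; A found path rebuilds a reused or spawned spline actor and updates the blackboard.
; Blocked endpoints retry with growing lateral, then vertical offsets bounded by attack range.
; An out-of-bounds start, missing path, or blocked start without a spline relocates the enemy to a random spawner.
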(event `self.ReceiveExecuteAI`
  (params (OwnerController :type "AIController Object Reference") (ControlledPawn :type "Pawn Object Reference"))
  (`KismetSystemLibrary.PrintText` "------------STARTED------------")
  (bind _asbp_flying_enemy_ai (cast `/Game/Blueprints/AI/BP_FlyingEnemyAI` ControlledPawn)
    (:`then`
      (set `self.ControlledPawn` _asbp_flying_enemy_ai)
      (cast `Actor` (`KismetSystemLibrary.Conv_InterfaceToObject` (`EnemyAI.GetTarget` _asbp_flying_enemy_ai))
        (:`then`
          (`KismetSystemLibrary.PrintText` "Cast to actor succeeded")
          (set `self.Owner Controller` OwnerController)
          (bind _controlledpawn (`self.ControlledPawn`)
            (:`then`
              (`KismetSystemLibrary.PrintText` "Controlled Pawn is valid")
              (set `self.CharacterMovementRef` (`Character.CharacterMovement` _controlledpawn))
              (`KismetSystemLibrary.PrintText` "Character Movement Ref is now set")
              (bind _returnvalue (`GameplayStatics.GetActorOfClass` "/Script/Navigation3D.NavigationVolume3D"))
              (`KismetSystemLibrary.PrintText` "Getting Navigation Volume 3D")
              (set `self.NavigationVolume3D` _returnvalue)
              (`KismetSystemLibrary.PrintText` "Navigation Volume 3D is now set")
              (bind _navigationvolume3d (`self.NavigationVolume3D`)
                (:`then`
                  (`KismetSystemLibrary.PrintText` "Navigation Volume 3D is valid")
                  (set `self.CurrentAttemptEndLocation` (`self.Get Target Location`))
                  (set `self.CurrentAttemptStartLocation` (`Actor.K2_GetActorLocation` (`self.ControlledPawn`)))
                  (`KismetSystemLibrary.PrintText` "Target Location fetched and set")
                  (set `self.ReadjustmentVerticalLength` 0.0)
                  (set `self.ReadjustmentLateralLength` 0.0)
                  (set `self.ReadjustmentIndex` 0)
                  (bind (_outpath _returnvalue_2) (`NavigationVolume3D.FindPath` _navigationvolume3d (`self.CurrentAttemptStartLocation`) (`self.CurrentAttemptEndLocation`)))
                  (switch `ENavigationVolumeResult` _returnvalue_2 :!label _label
                    (:`ENVR_Success`
                      (bind _returnvalue_3 (`|GetEnumeratorNameAsString` _returnvalue_2))
                      (`KismetSystemLibrary.PrintString` _returnvalue_3)
                      (`KismetSystemLibrary.PrintText` "Find Path found a path")
                      (set `self.Path` _outpath)
                      (`KismetSystemLibrary.PrintText` "Path local variable set")
                      (bind _asbp_flying_enemy_spline_path (cast `/Game/Blueprints/AI/BP_FlyingEnemySplinePath` (`BTFunctionLibrary.GetBlackboardValueAsActor` (`self.SplinePathKey`)))
                        (:`then`
                          (set `self.SplinePath` _asbp_flying_enemy_spline_path))
                        (:`CastFailed`
                          (bind _returnvalue_4 (`|SpawnActorFromClass` "/Game/Blueprints/AI/BP_FlyingEnemySplinePath.BP_FlyingEnemySplinePath_C" (`Actor.GetTransform` (`self.ControlledPawn`)) "AlwaysSpawn" "MultiplyWithRoot" null null))
                          (bind _output_get (set `self.SplinePath` _returnvalue_4))))
                      (bind _spline (`/Game/Blueprints/AI/BP_FlyingEnemySplinePath.Spline` _output_get))
                      (`SplineComponent.ClearSplinePoints` _spline true)
                      (for _array_element (`self.Path`)
                        (`SplineComponent.AddSplinePoint` _spline _array_element "World" true))
                      (`BTFunctionLibrary.SetBlackboardValueAsObject` (`self.SplinePathKey`) (`self.SplinePath`))
                      (`BTFunctionLibrary.SetBlackboardValueAsBool` (`self.PathNeedsRecalculationKey`))
                      (`BTFunctionLibrary.SetBlackboardValueAsFloat` (`self.DistanceAlongSpline`))
                      (`self.FinishExecute` true)
                      (`KismetSystemLibrary.PrintText` "------------FINISHED------------"))
                    (:`ENVR_StartNodeInvalid`
                      (`KismetSystemLibrary.PrintString` _returnvalue_3)
                      (`EnemySpawnManagerSubsystem.RelocateToRandomSpawner` (subsystem `EnemySpawnManagerSubsystem`) (`self.ControlledPawn`) :!label _label_2)
                      (`self.FinishExecute` true))
                    (:`ENVR_StartNodeBlocked`
                      (`/Engine/EditorBlueprintResources/StandardMacros.IsValid` (`self.SplinePath`)
                        (:`Is Valid`
                          (if (`self.StopAttempting`)
                            (`self.FinishExecute` false)
                            (else
                              (bind _output_get_2 (`self.ResolvePathCollision` (`self.CurrentAttemptStartLocation`)))
                              (set `self.CurrentAttemptStartLocation` _output_get_2)
                              (goto _label))))
                        (:`Is Not Valid`
                          (goto _label_2))))
                    (:`ENVR_EndNodeInvalid`
                      (`KismetSystemLibrary.PrintString` _returnvalue_3)
                      (`KismetSystemLibrary.PrintText` "End node of Path is invalid")
                      (`self.FinishExecute` false))
                    (:`ENVR_EndNodeBlocked`
                      (if (`self.StopAttempting`)
                        (`self.FinishExecute` false)
                        (else
                          (bind _output_get_3 (`self.ResolvePathCollision` (`self.CurrentAttemptEndLocation`)))
                          (set `self.CurrentAttemptEndLocation` _output_get_3)
                          (goto _label))))
                    (:`ENVR_NoPathExists`
                      (goto _label_2))
                    (:`ENVR_PathToSelf`
                      (`KismetSystemLibrary.PrintString` _returnvalue_3)
                      (`self.FinishExecute` true))
                    (:`ENVR_UnknownError`
                      (`KismetSystemLibrary.PrintString` _returnvalue_3)
                      (`KismetSystemLibrary.PrintText` "An unknown error occurred during path generation.")
                      (`self.FinishExecute` false))))
                (:`else`
                  (`self.FinishExecute` false)
                  (`KismetSystemLibrary.PrintText` "Navigation3D not valid"))))
            (:`else`
              (`self.FinishExecute` false)
              (`KismetSystemLibrary.PrintText` "ControlledPawn not valid"))))
        (:`CastFailed`
          (`KismetSystemLibrary.PrintText` "Cast to Actor failed")
          (`self.FinishExecute` false))))
    (:`CastFailed`
      (`KismetSystemLibrary.PrintText` "Cast to EnemyAI failed"))))

(fn `Get Target Location`
  (returns (`Target Location` :type "Vector Structure"))
  (bind _asactor (cast `Actor` (`KismetSystemLibrary.Conv_InterfaceToObject` (`EnemyAI.GetTarget` (`self.ControlledPawn`)))))
  (return (`Actor.K2_GetActorLocation` _asactor)))

(fn `ResolvePathCollision`
  (params (CollisionLocation :type "Vector Structure"))
  (returns (Output_Get :type "Vector Structure"))
  (locals (Location :type "Vector Structure"))
  (bind (_target_location_x _target_location_y _target_location_z) (`KismetMathLibrary.BreakVector` (`self.Get Target Location`)))
  (bind _returnvalue (+ (`self.ReadjustmentLateralLength`) (`self.ReadjustmentIncrease`)))
  (bind _returnvalue_2 (+ (`self.ReadjustmentVerticalLength`) (`self.ReadjustmentIncrease`)))
  (set `local.Location` CollisionLocation)
  (if (< (`self.ReadjustmentIndex`) (`KismetArrayLibrary.Array_Length` (`self.ReadjustmentOffsets`)))
    (set `local.Location` (+ (`local.Location`) (* (`|GetArrayItem` (`self.ReadjustmentOffsets`) (`self.ReadjustmentIndex`)) (`self.ReadjustmentLateralLength`))) :!label _label)
    (`/Engine/EditorBlueprintResources/StandardMacros.IncrementInt` (`self.ReadjustmentIndex`)
      (:`  `
        (return (`local.Location`))))
    (elif (<= _returnvalue (`EnemyAI.GetAttackRange` (`self.ControlledPawn`)))
      (set `self.ReadjustmentIndex` 0)
      (set `self.ReadjustmentLateralLength` _returnvalue)
      (goto _label)
      (elif (<= _returnvalue_2 (`EnemyAI.GetAttackRange` (`self.ControlledPawn`)))
        (bind _output_get (set `self.ReadjustmentVerticalLength` _returnvalue_2))
        (set `local.Location` (`KismetMathLibrary.MakeVector` _target_location_x _target_location_y (+ _output_get _target_location_z)))
        (return (`local.Location`))
        (else
          (`self.FinishExecute` false)
          (set `self.StopAttempting` true)
          (`KismetSystemLibrary.PrintText` "FINISH EXECUTE HAS RUN"))))))