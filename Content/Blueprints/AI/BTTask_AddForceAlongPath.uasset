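; Behavior tree task that moves a flying enemy AI through the points of a path read from a blackboard PathData object.
; It chains AIMoveTo calls without pathfinding, advancing the index on each finished move, then resets it and finishes successfully.
; Despite the task's name, no force is applied: helper functions for force, velocity limit and facing the goal are defined but never called.
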(event `self.ReceiveExecuteAI`
  (params (OwnerController :type "AIController Object Reference") (ControlledPawn :type "Pawn Object Reference"))
  ; Setup
  (set `self.Owner Controller` OwnerController)
  (bind _asbp_flying_enemy_ai (cast `/Game/Blueprints/AI/BP_FlyingEnemyAI` ControlledPawn))
  (set `self.ControlledCharacterRef` _asbp_flying_enemy_ai)
  (bind _aspath_data (cast `PathData` (`BTFunctionLibrary.GetBlackboardValueAsObject` (`self.PathKey`))))
  (set `self.Path` (`PathData.Path` _aspath_data))
  ; Add force toward target location
  (if (< (`self.Path Index`) (`KismetArrayLibrary.Array_Length` (`self.Path`))) :!label _label
    (`KismetSystemLibrary.PrintText` "True")
    (`AITask_MoveTo.AIMoveTo` (`self.Owner Controller`) (`|GetArrayItem` (`self.Path`) (`self.Path Index`)) null -1.0 "Disable" "Enable" false false false "Disable"
      (:`OnMoveFinished`
        (`/Engine/EditorBlueprintResources/StandardMacros.IncrementInt` (`self.Path Index`)
          (:`  `
            (goto _label)))))
    (else
      (set `self.Path Index` 0)
      (`KismetSystemLibrary.PrintText` "False")
      (`self.FinishExecute` true))))

(fn `BelowMaxVelocity?`
  (returns (`BelowMax?` :type Boolean))
  (bind _returnvalue (`PrimitiveComponent.GetPhysicsLinearVelocity` (`Character.CapsuleComponent` (`self.ControlledCharacterRef`)) "None"))
  (return (<= (`KismetMathLibrary.VSize` _returnvalue) (`self.MaxVelocity`))))

(fn `GetDistanceToGoal`
  (returns (Distance :type "Float (double-precision)"))
  (bind _controlledcharacterref (`self.ControlledCharacterRef`))
  (bind _goallocation (`self.GoalLocation`))
  (`/Engine/EditorBlueprintResources/StandardMacros.IsValid` _controlledcharacterref
    (:`Is Valid`
      (if (`AIBlueprintHelperLibrary.IsValidAILocation` _goallocation)
        (return (`KismetMathLibrary.VSize` (- (`Actor.K2_GetActorLocation` _controlledcharacterref) _goallocation)))))))

(fn `GetForceVector`
  (returns (ReturnValue :type "Vector Structure"))
  (return (* (`KismetMathLibrary.VLerp` (`KismetMathLibrary.GetDirectionUnitVector` (`Actor.K2_GetActorLocation` (`self.ControlledCharacterRef`)) (`self.GoalLocation`)) (0.0 0.0 0.0) (/ (- (`self.InitialDistance`) (`self.GetDistanceToGoal`)) (`self.InitialDistance`))) (`self.Acceleration`))))

(fn `UpdateRotationToFaceVelocity`
  (`Actor.K2_SetActorRotation` (`self.ControlledCharacterRef`) (`KismetMathLibrary.RLerp` (`Actor.K2_GetActorRotation` (`self.ControlledCharacterRef`)) (`KismetMathLibrary.FindLookAtRotation` (`Actor.K2_GetActorLocation` (`self.ControlledCharacterRef`)) (`self.GoalLocation`)) (`self.RotationAlpha`) true) false))