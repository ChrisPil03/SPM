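; BP_WaspProjectile is the projectile actor for a Wasp AI attack, damaging what it hits through the Gameplay Ability System.
; On sphere overlap, it checks whether the hit actor implements the Attackable interface and, if so, has its owning gameplay ability apply the damage effect to that target.
; Every overlap, valid target or not, ends that ability and destroys the projectile.
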(event `self.ReceiveBeginPlay`
  (add `PrimitiveComponent.OnComponentBeginOverlap` (`self.Sphere`) (delegate `OnComponentBeginOverlap_Event`)))

(event `OnComponentBeginOverlap_Event`
  (params (OverlappedComponent :type "PrimitiveComponent Object Reference") (OtherActor :type "Actor Object Reference") (OtherComp :type "PrimitiveComponent Object Reference") (OtherBodyIndex :type Integer) (bFromSweep :type Boolean) (SweepResult :type "HitResult Structure (by ref)"))
  (`/Engine/EditorBlueprintResources/StandardMacros.IsValid` OtherActor
    (:`Is Valid`
      (set `self.HitTarget` OtherActor)
      (if (`KismetSystemLibrary.DoesImplementInterface` (`self.HitTarget`) "/Script/CoolGang.Attackable")
        (`GameplayAbility.BP_ApplyGameplayEffectToTarget` (`self.ProjectileGameplayAbility`) (`AbilitySystemBlueprintLibrary.AbilityTargetDataFromActor` (`self.HitTarget`)) (`self.ProjectileDamageEffect`) 1 1)
        (`self.EndAndDestroy`)
        (else
          (`self.EndAndDestroy`))))
    (:`Is Not Valid`
      (`self.EndAndDestroy`))))

(fn `EndAndDestroy`
  (`GameplayAbility.K2_EndAbility` (`self.ProjectileGameplayAbility`))
  (`self.K2_DestroyActor`))

(fn `UserConstructionScript`)