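; BP_NavLinks is a smart nav link that makes BP_GroundEnemyAI agents jump to the link's destination.
; On SmartLinkReached, it derives an arc parameter from the jump's vertical direction, stopping movement first for level or upward jumps.
; That parameter shapes a suggested projectile velocity and its gravity override, then the enemy receives the link and jumping state.
; A separate InitiateLaunch event launches the enemy and clears the link.
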(event `self.ReceiveSmartLinkReached`
  (params (Agent :type "Actor Object Reference") (Destination :type "Vector Structure"))
  (bind _asbp_ground_enemy_ai (cast `/Game/Blueprints/AI/BP_GroundEnemyAI` Agent))
  (set `self.Enemy` _asbp_ground_enemy_ai)
  (bind _returnvalue (`Actor.K2_GetActorLocation` _asbp_ground_enemy_ai))
  (bind (_returnvalue_x _returnvalue_y _returnvalue_z) (`KismetMathLibrary.BreakVector` (`KismetMathLibrary.Normal` (- Destination _returnvalue))))
  (if (< _returnvalue_z 0.0)
    (bind _output_get (set `self.Arc Param` (* (`KismetMathLibrary.Abs` _returnvalue_z) 0.8)))
    (if (>= _output_get 0.0)
      (bind _outlaunchvelocity (`GameplayStatics.SuggestProjectileVelocity_CustomArc` _returnvalue Destination (`KismetMathLibrary.Lerp` -6000.0 -12000.0 (`self.Arc Param`)) (`self.Arc Param`) :!label _label))
      (set `self.Out Launch Velocity` _outlaunchvelocity)
      (`/Game/Blueprints/AI/BP_GroundEnemyAI.SetCurrentNavLink` (`self.Enemy`) self)
      (`EnemyAI.SetJumpingState` (`self.Enemy`) true))
    (else
      (bind _output_get_2 (set `self.Arc Param` (* (- 1.0 _returnvalue_z) 1.5)))
      (if (>= _output_get_2 0.0)
        (`MovementComponent.StopMovementImmediately` (`Character.CharacterMovement` (`self.Enemy`)))
        (goto _label)))))

(event `InitiateLaunch`
  (`Character.LaunchCharacter` (`self.Enemy`) (`self.Out Launch Velocity`) true true)
  (`/Game/Blueprints/AI/BP_GroundEnemyAI.SetCurrentNavLink` (`self.Enemy`) null))