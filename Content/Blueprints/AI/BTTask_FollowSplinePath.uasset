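; Behavior tree task that moves a flying enemy along a BP_FlyingEnemySplinePath taken from the blackboard.
; Each tick advances the blackboard distance along the spline, sets the pawn's movement velocity directly, then finishes successfully.
; Velocity follows the unnormalized vector between spline points two indices apart to straighten the path.
; When that look-ahead is invalid, it steers toward the spline point at the current distance and draws a debug arrow.
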(event `self.ReceiveTick`
  (params (OwnerActor :type "Actor Object Reference") (DeltaSeconds :type "Float (single-precision)"))
  (bind _returnvalue_location (`KismetMathLibrary.BreakTransform` (`SplineComponent.GetTransformAtDistanceAlongSpline` (`self.SplineComponent`) (`BTFunctionLibrary.GetBlackboardValueAsFloat` (`self.DistanceAlongSpline`)) "World" false)))
  (bind _returnvalue (`Controller.K2_GetPawn` (`AIBlueprintHelperLibrary.GetAIController` (`self.Owner Actor`))))
  (bind _returnvalue_2 (`Pawn.GetMovementComponent` _returnvalue))
  (bind _returnvalue_3 (`KismetMathLibrary.GetDirectionUnitVector` (`self.EnemyLocation`) _returnvalue_location))
  (set `self.Owner Actor` OwnerActor)
  (set `self.Delta Seconds` DeltaSeconds)
  (`BTFunctionLibrary.SetBlackboardValueAsFloat` (`self.DistanceAlongSpline`) (+ (* (`self.MovementSpeed`) (`self.Delta Seconds`)) (`BTFunctionLibrary.GetBlackboardValueAsFloat` (`self.DistanceAlongSpline`))))
  (bind _asbp_flying_enemy_spline_path (cast `/Game/Blueprints/AI/BP_FlyingEnemySplinePath` (`BTFunctionLibrary.GetBlackboardValueAsActor` (`self.SplinePathKey`))))
  (set `self.SplineComponent` (`/Game/Blueprints/AI/BP_FlyingEnemySplinePath.Spline` _asbp_flying_enemy_spline_path))
  (set `self.EnemyLocation` (`Actor.K2_GetActorLocation` _returnvalue))
  (bind (_straighteneddirection _isvalid) (`self.GetStraightenedDirection` (`self.SplineComponent`) (`KismetMathLibrary.FCeil` (`SplineComponent.GetInputKeyValueAtDistanceAlongSpline` (`self.SplineComponent`) (`BTFunctionLibrary.GetBlackboardValueAsFloat` (`self.DistanceAlongSpline`)))) 2))
  (if _isvalid
    (set `MovementComponent.Velocity` (* _straighteneddirection (`self.SmoothSplineMovementSpeed`)) _returnvalue_2)
    (else
      (`KismetSystemLibrary.DrawDebugArrow` (`self.EnemyLocation`) (+ (`self.EnemyLocation`) (* _returnvalue_3 (`self.MovementSpeed`))) 50.0 (struct :`R` 1.0 :`G` 0.137932 :`A` 1.0) 0.1 5.0)
      (set `MovementComponent.Velocity` (* _returnvalue_3 (`self.MovementSpeed`)) _returnvalue_2)))
  (`self.FinishExecute` true))

(fn `GetStraightenedDirection`
  (params (SplineCompRef :type "SplineComponent Object Reference") (StartIndex :type Integer) (LookAheadAmount :type Integer))
  (returns (StraightenedDirection :type "Vector Structure") (IsValid :type Boolean))
  (locals (SplineComp :type "SplineComponent Object Reference") (FowardIndex :type Integer) (CurrentIndex :type Integer) (RawDirection :type "Vector Structure") (CalcIsValid :type Boolean :default false))
  (bind _returnvalue (- (`SplineComponent.GetLocationAtSplinePoint` (`local.SplineComp`) (`local.FowardIndex`) "World") (`SplineComponent.GetLocationAtSplinePoint` (`local.SplineComp`) (`local.CurrentIndex`) "World")))
  (bind _output_get (set `local.CurrentIndex` StartIndex))
  (set `local.FowardIndex` (+ _output_get LookAheadAmount))
  (bind _output_get_2 (set `local.SplineComp` SplineCompRef))
  (`/Engine/EditorBlueprintResources/StandardMacros.IsValid` _output_get_2
    (:`Is Valid`
      (if (< (`local.FowardIndex`) (`SplineComponent.GetNumberOfSplinePoints` (`local.SplineComp`)))
        (if (== _returnvalue (0.0 0.0 0.0) :`ErrorTolerance` 5.0)
          (return (0.0 0.0 0.0) false)
          (else
            (return _returnvalue true)))
        (else
          (return (0.0 0.0 0.0) false))))
    (:`Is Not Valid`
      (return (0.0 0.0 0.0) false))))