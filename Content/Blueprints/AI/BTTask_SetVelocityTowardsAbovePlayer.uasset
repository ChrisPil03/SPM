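; Behavior tree task that steers an AI character toward a point a set height above the player.
; It writes CharacterMovement velocity directly, aimed from the pawn to the player's location plus ElevationHeight and scaled by Speed.
; Velocity is zeroed when the pawn is within a fixed tolerance of that point, and the task finishes successfully right away without waiting for arrival.
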(event `self.ReceiveExecuteAI`
  (params (OwnerController :type "AIController Object Reference") (ControlledPawn :type "Pawn Object Reference"))
  (bind (_from _to) (`self.GetStartAndGoal`))
  (bind (_from_2 _to_2) (`self.GetStartAndGoal`))
  (bind _output_get (set `self.ControlledPawn` ControlledPawn))
  (bind _ascharacter (cast `Character` _output_get))
  (set `self.CharacterMovementRef` (`Character.CharacterMovement` _ascharacter))
  (if (== _from _to :`ErrorTolerance` 300.0)
    (set `MovementComponent.Velocity` (0.0 0.0 0.0) (`self.CharacterMovementRef`))
    (else
      (set `MovementComponent.Velocity` (* (`KismetMathLibrary.GetDirectionUnitVector` _from_2 _to_2) (`KismetMathLibrary.Conv_DoubleToVector` (`self.Speed`))) (`self.CharacterMovementRef`))))
  (`self.FinishExecute` true))

(fn `GetStartAndGoal`
  (returns (From :type "Vector Structure") (To :type "Vector Structure"))
  (return (`Actor.K2_GetActorLocation` (`self.ControlledPawn`)) (+ (`Actor.K2_GetActorLocation` (`GameplayStatics.GetPlayerCharacter` 0)) (`KismetMathLibrary.MakeVector` 0.0 0.0 (`self.ElevationHeight`)))))