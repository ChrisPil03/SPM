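; Base enemy AI character Blueprint that pursues either the player or an objective, with attack range and walk speed set per target type.
; Target change events apply those values, and an in-range flag switches between near-target and stored target speed.
; Tick rotates it toward its current target.
; Weapon damage spawns a damage amount actor, and pre-death plays a sound and calls Die only when DeathSound is valid.
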(event `self.PerformPreDeathActions`
  (params (DeathCauser :type "Actor Object Reference"))
  (bind _deathsound (`self.DeathSound`))
  (`/Engine/EditorBlueprintResources/StandardMacros.IsValid` _deathsound
    (:`Is Valid`
      (`GameplayStatics.PlaySoundAtLocation` _deathsound (`self.K2_GetActorLocation`) (struct) 1.0 1.0 0.0 null null null null)
      (`self.Die`))))

(event `self.ReceiveTick`
  (params (DeltaSeconds :type "Float (single-precision)"))
  (bind _asactor (cast `Actor` (`KismetSystemLibrary.Conv_InterfaceToObject` (`self.GetTarget`))))
  (`/Engine/EditorBlueprintResources/StandardMacros.IsValid` _asactor
    (:`Is Valid`
      (bind (_returnvalue_roll _returnvalue_pitch _returnvalue_yaw) (`KismetMathLibrary.BreakRotator` (`KismetMathLibrary.FindLookAtRotation` (`self.K2_GetActorLocation` self) (`self.K2_GetActorLocation` _asactor))))
      (`self.K2_SetActorRotation` self (`KismetMathLibrary.MakeRotator` _returnvalue_roll 0.0 _returnvalue_yaw) false))))

(event `self.ReceiveAnyDamage`
  (params (Damage :type "Float (single-precision)") (DamageType :type "DamageType Object Reference") (InstigatedBy :type "Controller Object Reference") (DamageCauser :type "Actor Object Reference"))
  (cast `/Game/Blueprints/Weapons/BP_Weapon` DamageCauser)
  (bind _asbp_player_character (cast `/Game/Blueprints/BP_PlayerCharacter` (`GameplayStatics.GetPlayerCharacter` 0)))
  (`|SpawnActorFromClass` "/Game/Blueprints/Widgets/UI_Blueprints/BP_DamageAmount.BP_DamageAmount_C" (`self.GetTransform`) "Undefined" "MultiplyWithRoot" null Damage self _asbp_player_character null))

(event `self.OnTargetChanged`
  (params (Target :type "Actor Object Reference"))
  (if (== Target (`GameplayStatics.GetPlayerCharacter` 0))
    (set `self.AttackRange` (`self.PlayerAttackRange`))
    (bind _output_get (set `CharacterMovementComponent.MaxWalkSpeed` (`self.MovementSpeedAgainstPlayer`) (`self.CharacterMovement`)))
    (set `self.CurrentTargetMovementSpeed` _output_get)
    (else
      (set `self.AttackRange` (`self.ObjectiveAttackRange`))
      (bind _output_get_2 (set `CharacterMovementComponent.MaxWalkSpeed` (`self.MovementSpeedAgainstObjective`) (`self.CharacterMovement`)))
      (set `self.CurrentTargetMovementSpeed` _output_get_2))))

(event `self.SetTargetInRange`
  (params (IsInRange :type Boolean))
  (bind _output_get (set `self.bTargetInRange` IsInRange))
  (if _output_get
    (set `CharacterMovementComponent.MaxWalkSpeed` (`self.MovementSpeedNearTarget`) (`self.CharacterMovement`))
    (else
      (set `CharacterMovementComponent.MaxWalkSpeed` (`self.CurrentTargetMovementSpeed`) (`self.CharacterMovement`)))))

(fn `UserConstructionScript`)