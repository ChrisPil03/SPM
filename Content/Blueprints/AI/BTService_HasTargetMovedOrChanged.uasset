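; Behavior tree service that flags an enemy AI's path for recalculation when its target changes or moves too far.
; Each tick it compares the blackboard target with the EnemyAI's own target.
; If unchanged, it picks a close, medium or far movement threshold by squared distance to the target.
; It requests recalculation when that threshold shrinks or the target's squared displacement from its stored previous position reaches it.
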(event `self.ReceiveTickAI`
  (params (OwnerController :type "AIController Object Reference") (ControlledPawn :type "Pawn Object Reference") (DeltaSeconds :type "Float (single-precision)"))
  (bind _closedistance (`self.CloseDistance`))
  (bind _mediumdistance (`self.MediumDistance`))
  (bind _movementthreshold (`self.MovementThreshold`))
  (bind _returnvalue (!= (`self.Target`) (`KismetSystemLibrary.Conv_InterfaceToObject` (`EnemyAI.GetTarget` (`self.Enemy AI`)))))
  (bind _asenemy_ai (cast `EnemyAI` ControlledPawn))
  (set `self.Enemy AI` _asenemy_ai)
  (bind _output_get (set `self.Target` (`BTFunctionLibrary.GetBlackboardValueAsActor` (`self.TargetActorKey`))))
  (`/Engine/EditorBlueprintResources/StandardMacros.IsValid` _output_get
    (:`Is Valid`
      (`BTFunctionLibrary.SetBlackboardValueAsBool` (`self.PathNeedsRecalculationKey`) _returnvalue)
      (if (not _returnvalue)
        (set `self.DistanceToTargetSquared` (`KismetMathLibrary.Vector_DistanceSquared` (`Actor.GetActorBounds` (`self.Enemy AI`) false false) (`Actor.GetActorBounds` (`self.Target`) false false)))
        (set `self.DistanceMovedSquared` (`KismetMathLibrary.Vector_DistanceSquared` (`BTFunctionLibrary.GetBlackboardValueAsVector` (`self.PreviousPosition`)) (`Actor.GetActorBounds` (`self.Target`) false false)))
        (if (== (`KismetMathLibrary.SelectFloat` (`self.CloseMovementThreshold`) (`self.MediumDistanceMovementThreshold`) (<= (`self.DistanceToTargetSquared`) (* _closedistance _closedistance))) (`self.CloseMovementThreshold`))
          (set `self.MovementThreshold` (`self.CloseMovementThreshold`))
          (elif (== (`KismetMathLibrary.SelectFloat` (`self.MediumDistanceMovementThreshold`) (`self.FarMovementThreshold`) (<= (`self.DistanceToTargetSquared`) (* _mediumdistance _mediumdistance))) (`self.MediumDistanceMovementThreshold`))
            (set `self.MovementThreshold` (`self.MediumDistanceMovementThreshold`))
            (else
              (set `self.MovementThreshold` (`self.FarMovementThreshold`)))))
        (if (> (`BTFunctionLibrary.GetBlackboardValueAsFloat` (`self.PreviousMovementThreshold`)) (`self.MovementThreshold`))
          (`BTFunctionLibrary.SetBlackboardValueAsBool` (`self.PathNeedsRecalculationKey`) true)
          (else
            (`BTFunctionLibrary.SetBlackboardValueAsBool` (`self.PathNeedsRecalculationKey`) (>= (`self.DistanceMovedSquared`) (* _movementthreshold _movementthreshold)))))
        (`BTFunctionLibrary.SetBlackboardValueAsFloat` (`self.PreviousMovementThreshold`) (`self.MovementThreshold`))))))