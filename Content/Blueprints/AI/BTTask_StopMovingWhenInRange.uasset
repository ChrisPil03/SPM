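; Behavior tree task that conditionally halts an enemy AI pawn, based on attack range and target distance.
; It compares the BP_EnemyAIBase attack range with the DistanceToTargetSquared blackboard value, and when the range is less than or equal to it, zeroes movement velocity and succeeds.
; Otherwise the task fails; a failed cast leaves it unfinished.
; Despite the name, the stop fires when that stored distance is at or beyond the range value.
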(event `self.ReceiveExecuteAI`
  (params (OwnerController :type "AIController Object Reference") (ControlledPawn :type "Pawn Object Reference"))
  (set `self.Controlled Pawn` ControlledPawn)
  (bind _asbp_enemy_aibase (cast `/Game/Blueprints/AI/BP_EnemyAIBase` (`self.Controlled Pawn`)))
  (if (<= (`EnemyAI.GetAttackRange` _asbp_enemy_aibase) (`BTFunctionLibrary.GetBlackboardValueAsFloat` (`self.DistanceToTargetSquared`)))
    (set `MovementComponent.Velocity` (0.0 0.0 0.0) (`Pawn.GetMovementComponent` (`self.Controlled Pawn`)))
    (`self.FinishExecute` true)
    (else
      (`self.FinishExecute` false))))