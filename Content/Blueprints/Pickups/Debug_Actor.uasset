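; Debug actor that flies from its spawn location to the player pawn's starting position when play begins.
; BeginPlay caches both locations and draws debug spheres at each for ten seconds.
; A timeline float track then drives a vector lerp between them, setting the actor's location without sweep and printing the alpha and interpolated position every update.
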(event `self.ReceiveBeginPlay`
  (bind _returnvalue (`self.K2_GetActorLocation` (`GameplayStatics.GetPlayerPawn` 0)))
  (bind _output_get (set `self.NewVar` (`self.K2_GetActorLocation`)))
  (set `self.NewVar_0` _returnvalue)
  (`KismetSystemLibrary.DrawDebugSphere` _output_get 100.0 12 (struct :`R` 1.0 :`B` 0.49937 :`A` 1.0) 10.0)
  (`KismetSystemLibrary.DrawDebugSphere` _returnvalue 100.0 12 (struct :`R` 1.0 :`A` 1.0) 10.0)
  (bind (_direction _newtrack_0) (`Timeline|Timeline`)
    (:`Update`
      (`KismetSystemLibrary.PrintString` (`KismetStringLibrary.Conv_DoubleToString` _newtrack_0))
      (bind _returnvalue_2 (`KismetMathLibrary.VLerp` (`self.NewVar`) (`self.NewVar_0`) _newtrack_0))
      (`KismetSystemLibrary.PrintString` (`KismetStringLibrary.Conv_VectorToString` _returnvalue_2))
      (`self.K2_SetActorLocation` _returnvalue_2))))

(fn `UserConstructionScript`)