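; Base pickup actor that grants a random gameplay-effect upgrade to one of the player's guns.
; On BeginPlay it picks a random gun from player pawn 0 and a random effect, then applies that gun's pickup material to its cube.
; The cube spins on Tick; player overlap applies the effect to the gun's Ability System Component and destroys the pickup.
; Several bobbing-motion experiments remain disconnected.
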(event `self.ReceiveBeginPlay`
  (bind _gun (`self.Gun`))
  (set `self.StartLocation` (`SceneComponent.RelativeLocation` (`self.Cube`)))
  (`|ExecutionSequence`
    (:`then_0`
      (bind _asbp_player_character (cast `/Game/Blueprints/BP_PlayerCharacter` (`GameplayStatics.GetPlayerPawn` 0)))
      (set `self.Gun` (`KismetArrayLibrary.Array_Random` (`PlayerCharacter.Guns` _asbp_player_character))))
    (:`then_1`
      (set `self.Upgrade` (`KismetArrayLibrary.Array_Random` (`self.UpgradeGameplayEffectsArray`))))
    (:`then_2`
      (`/Engine/EditorBlueprintResources/StandardMacros.IsValid` _gun
        (:`Is Valid`
          (`PrimitiveComponent.SetMaterial` (`self.Cube`) 1 (`GunBase.PickupMat` _gun)))))
    (:`then_3`
      (`KismetSystemLibrary.PrintString` (`KismetStringLibrary.Concat_StrStr` "Weapon to upgrade: " (`KismetSystemLibrary.GetDisplayName` (`self.Gun`))))
      (`KismetSystemLibrary.PrintString` (`KismetStringLibrary.Concat_StrStr` "upgrade: " (`KismetSystemLibrary.GetClassDisplayName` (`self.Upgrade`)))))))

(event `self.ReceiveTick`
  (params (DeltaSeconds :type "Float (single-precision)"))
  (`|ExecutionSequence`
    (:`then_0`
      (`SceneComponent.K2_AddLocalRotation` (`self.Cube`) (`KismetMathLibrary.MakeRotator` 0.0 0.0 (* DeltaSeconds (`self.Rotate speed`))) false false))))

(event `self.ReceiveActorBeginOverlap`
  (params (OtherActor :type "Actor Object Reference"))
  (cast `/Game/Blueprints/BP_PlayerCharacter` OtherActor)
  (`AbilitySystemComponent.BP_ApplyGameplayEffectToTarget` :`self` (`self.AbilitySystem`) :`GameplayEffectClass` (`self.Upgrade`) :`Target` (`AbilitySystemBlueprintLibrary.GetAbilitySystemComponent` (`self.Gun`)))
  (`self.K2_DestroyActor`))

(fn `UserConstructionScript`)