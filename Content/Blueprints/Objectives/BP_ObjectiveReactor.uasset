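; Reactor objective actor that drives the visual state of its shield as it takes damage, breaks and is restored.
; On BeginPlay it creates dynamic materials for the base and random shield meshes, then pushes shield percentage into their HP parameter on change.
; Shield destruction and objective completion play break and restore timelines, animating both materials' Broken values and a Material Parameter Collection radius for the light sphere.
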(event `self.ReceiveBeginPlay`
  (`self.SetMaterialInstances`)
  (add `self.OnShieldChanged` (delegate `OnShieldChangedEvent`))
  (add `self.OnShieldDestroyed` (delegate `OnShieldDestroyedEvent`))
  (add `ObjectiveBase.OnObjectiveCompleted` (delegate `OnObjectiveCompletedEvent`)))

(event `OnShieldChangedEvent`
  (`self.SetHPMaterialValues`))

(event `OnObjectiveCompletedEvent`
  (bind (_direction _bsaetrack _randomtrack _lightspheretrack) (`Timeline|ShieldRestoreTimeline` :!via `PlayFromStart`)
    (:`Update`
      (`MaterialInstanceDynamic.SetScalarParameterValue` (`self.BaseMaterialInstance`) "Broken" _bsaetrack)
      (`MaterialInstanceDynamic.SetScalarParameterValue` (`self.RandomMaterialInstance`) "Broken" _randomtrack)
      (`KismetMaterialLibrary.SetScalarParameterValue` (`self.MPC`) (`self.RadiusName`) _lightspheretrack))))

(event `OnShieldDestroyedEvent`
  (bind (_direction _bsaetrack _randomtrack _lightspheretrack) (`Timeline|ShieldBreakTimeline` :!via `PlayFromStart`)
    (:`Update`
      (`MaterialInstanceDynamic.SetScalarParameterValue` (`self.BaseMaterialInstance`) "Broken" _bsaetrack)
      (`MaterialInstanceDynamic.SetScalarParameterValue` (`self.RandomMaterialInstance`) "Broken" _randomtrack)
      (`KismetMaterialLibrary.SetScalarParameterValue` (`self.MPC`) (`self.RadiusName`) _lightspheretrack))))

(fn `CreateAndSetProgressMaterial`
  (bind _returnvalue (`KismetMaterialLibrary.CreateDynamicMaterialInstance` (`PrimitiveComponent.GetMaterial` (`self.MeshComponent`) 0)))
  (bind _output_get (set `self.MaterialInstanceReference` _returnvalue))
  (`PrimitiveComponent.SetMaterial` (`self.MeshComponent`) 0 _output_get)
  (`MaterialInstanceDynamic.SetScalarParameterValue` (`self.MaterialInstanceReference`) "Fade Amount" 1.0))

(fn `SetHPMaterialValues`
  (bind _returnvalue (`self.GetShieldPercentage`))
  (`MaterialInstanceDynamic.SetScalarParameterValue` (`self.BaseMaterialInstance`) "HP" _returnvalue)
  (`MaterialInstanceDynamic.SetScalarParameterValue` (`self.RandomMaterialInstance`) "HP" _returnvalue))

(fn `SetMaterialInstances`
  (bind _returnvalue (`KismetMaterialLibrary.CreateDynamicMaterialInstance` (`PrimitiveComponent.GetMaterial` (`self.SM_ShieldBase`) 0)))
  (bind _output_get (set `self.BaseMaterialInstance` _returnvalue))
  (`PrimitiveComponent.SetMaterial` (`self.SM_ShieldBase`) 0 _output_get)
  (bind _returnvalue_2 (`KismetMaterialLibrary.CreateDynamicMaterialInstance` (`PrimitiveComponent.GetMaterial` (`self.SM_ShieldRandom`) 0)))
  (bind _output_get_2 (set `self.RandomMaterialInstance` _returnvalue_2))
  (`PrimitiveComponent.SetMaterial` (`self.SM_ShieldRandom`) 0 _output_get_2))

(fn `SetMaterialProgress`
  (params (Value :type "Float (single-precision)"))
  (`MaterialInstanceDynamic.SetScalarParameterValue` (`self.MaterialInstanceReference`) "Fade Amount" Value))

(fn `UserConstructionScript`)