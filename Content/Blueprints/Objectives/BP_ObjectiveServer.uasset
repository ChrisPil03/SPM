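; BP_ObjectiveServer is an interactable objective server that shows a malfunction state through its material and plays a sound when interacted with.
; On BeginPlay it creates dynamic material instances for a faded-out paused cable and the server, applying the server one to its mesh, and binds its interact delegate.
; SetServerLightColor toggles the server material's "Is Paused" parameter to reflect whether it is malfunctioning.
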(event `self.ReceiveBeginPlay`
  (`self.CreateMaterialsToSet`)
  (add `self.InteractDelegate` (delegate `InteractDelegate_Event`)))

(event `InteractDelegate_Event` :!signature `self.InteractDelegate`
  (params (Object :type "InteractableObject Object Reference"))
  (`GameplayStatics.PlaySoundAtLocation` "/Game/Audio/SoundCues/Objectives/SC_Interact.SC_Interact" (`SceneComponent.K2_GetComponentLocation` (`self.RootComponent`)) (struct) 1.0 1.0 0.0 null null null null))

(event `self.SetServerLightColor`
  (params (bMalfunctioning :type Boolean))
  (bind _servermaterialinstance (`self.ServerMaterialInstance`))
  (`/Engine/EditorBlueprintResources/StandardMacros.IsValid` _servermaterialinstance
    (:`Is Valid`
      (if bMalfunctioning
        (`MaterialInstanceDynamic.SetScalarParameterValue` _servermaterialinstance "Is Paused" 0.0)
        (else
          (`MaterialInstanceDynamic.SetScalarParameterValue` _servermaterialinstance "Is Paused" 1.0))))))

(fn `CreateMaterialsToSet`
  (bind _mesh (`self.Mesh`))
  (bind _returnvalue (`KismetMaterialLibrary.CreateDynamicMaterialInstance` (`self.CableMaterialToSet`)))
  (bind _output_get (set `self.CablePausedMaterial` _returnvalue))
  (`MaterialInstanceDynamic.SetScalarParameterValue` _output_get "Fade Amount" 0.0)
  (bind _returnvalue_2 (`KismetMaterialLibrary.CreateDynamicMaterialInstance` (`self.ServerMaterialToSet`)))
  (bind _output_get_2 (set `self.ServerMaterialInstance` _returnvalue_2))
  (`/Engine/EditorBlueprintResources/StandardMacros.IsValid` _mesh
    (:`Is Valid`
      (`PrimitiveComponent.SetMaterial` _mesh 0 _output_get_2))))

(fn `UserConstructionScript`)