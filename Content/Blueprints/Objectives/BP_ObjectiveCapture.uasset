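; BP_ObjectiveCapture is a capture objective that manages the visual lifecycle of a download zone around itself.
; Its events spawn an offset BP_DownloadZone attached to the objective and scaled from CaptureRadius to match the capture diameter, then later destroy it.
; Updates pass objective progress to the zone's ring size, flagged as growing only while the objective is in progress and a player is inside.
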(event `self.SpawnCaptureZone`
  ; Spawn Download Zone
  (bind _scale (`self.GetDownloadZoneScale`))
  (bind _returnvalue (`|SpawnActorFromClass` "/Game/Blueprints/VFX_BP/BP_DownloadZone.BP_DownloadZone_C" (`KismetMathLibrary.MakeTransform` (+ (`self.LocationOffset`) (`self.K2_GetActorLocation`)) (struct) _scale) "Undefined" "MultiplyWithRoot" null null))
  (bind _output_get (set `self.DownloadZone` _returnvalue))
  (`self.K2_AttachToActor` _output_get self "None" "KeepWorld" "KeepWorld" "KeepWorld" true))

(event `self.UpdateCaptureZoneSize`
  (bind _downloadzone (`self.DownloadZone`))
  ; Update Download Zone Size
  (if (`KismetSystemLibrary.IsValid` _downloadzone)
    (`/Game/Blueprints/VFX_BP/BP_DownloadZone.UpdateRingSize` _downloadzone (`self.GetObjectiveProgress`) (and (`self.GetIsInProgress`) (`self.GetIsPlayerInZone`)))))

(event `self.DestroyCaptureZone`
  (bind _downloadzone (`self.DownloadZone`))
  ; Destroy Download Zone
  (if (`KismetSystemLibrary.IsValid` _downloadzone)
    (`self.K2_DestroyActor` _downloadzone)
    (else
      (`KismetSystemLibrary.PrintString` "Destroy: Download Zone not valid"))))

(fn `GetDownloadZoneScale`
  (returns (Scale :type "Vector Structure"))
  (bind _returnvalue (* (/ (`self.CaptureRadius`) 100.0) 2.0))
  (return (`KismetMathLibrary.MakeVector` _returnvalue _returnvalue (`self.Spawn Transform Scale Z`))))

(fn `UserConstructionScript`)