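; BP_ObjectiveDefendGenerator is a defend-the-generator objective that shows the generator's health through its mesh material.
; On BeginPlay it creates a dynamic instance of the mesh's first material, applies it and starts the "Fade Amount" parameter at full.
; While the objective is active, Tick sets that parameter from the health percentage, with no other objective logic in this graph.
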(event `self.ReceiveBeginPlay`
  ; Begin Play
  (bind _returnvalue (`KismetMaterialLibrary.CreateDynamicMaterialInstance` (`PrimitiveComponent.GetMaterial` (`self.MeshComponent`) 0)))
  (bind _output_get (set `self.MaterialInstanceReference` _returnvalue))
  (`PrimitiveComponent.SetMaterial` (`self.MeshComponent`) 0 _output_get)
  (`MaterialInstanceDynamic.SetScalarParameterValue` (`self.MaterialInstanceReference`) "Fade Amount" 1.0))

(event `self.ReceiveTick`
  (params (DeltaSeconds :type "Float (single-precision)"))
  (if (`self.GetIsActive`)
    (`MaterialInstanceDynamic.SetScalarParameterValue` (`self.MaterialInstanceReference`) "Fade Amount" (`self.GetHealthPercentage`))))

(fn `UserConstructionScript`)