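; Interactable control panel objective that starts the active game when the player uses it.
; On BeginPlay it creates dynamic materials for module and screen, enables interaction and binds its delegates; activation sets scalar parameters on both materials.
; Interacting sets BP_DiveGameMode active, gives the player pistol, shotgun and rifle, equips the first, triggers a wireframe load, destroys the panel and starts in-game music through the GameInstance.
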(event `self.ReceiveBeginPlay`
  (`parent.ReceiveBeginPlay`)
  (`self.CreateSetMaterialInstance`)
  (add `self.InteractDelegate` (delegate `OnInteractEvent`))
  (add `self.OnActivated` (delegate `OnActivatedEvent`))
  (`self.SetCanInteractWith` true))

(event `OnActivatedEvent`
  (`MaterialInstanceDynamic.SetScalarParameterValue` (`self.ModuleMaterialInstance`) "Is Paused" 1.0)
  (`MaterialInstanceDynamic.SetScalarParameterValue` (`self.ScreenMaterialInstance`) "Activated" 1.0))

(event `OnInteractEvent` :!signature `self.InteractDelegate`
  (params (Object :type "InteractableObject Object Reference"))
  (bind _asbp_dive_game_mode (cast `/Game/Blueprints/BP_DiveGameMode` (`GameplayStatics.GetGameMode`)))
  (`CyberWarriorGameModeBase.SetGameActiveState` _asbp_dive_game_mode true)
  (bind _asbp_player_character (cast `/Game/Blueprints/BP_PlayerCharacter` (`GameplayStatics.GetPlayerPawn` 0)))
  (`|ExecutionSequence`
    (:`then_0`
      (`PlayerCharacter.GiveGun` _asbp_player_character "/Game/Blueprints/Weapons/BP_Pistol.BP_Pistol_C"))
    (:`then_1`
      (`PlayerCharacter.GiveGun` _asbp_player_character "/Game/Blueprints/Weapons/BP_Shotgun.BP_Shotgun_C"))
    (:`then_2`
      (`PlayerCharacter.GiveGun` _asbp_player_character "/Game/Blueprints/Weapons/BP_Rifle.BP_Rifle_C"))
    (:`then_3`
      (`PlayerCharacter.ChangeEquippedGun` _asbp_player_character 0))
    (:`then_4`
      (`/Game/Blueprints/VFX_BP/BP_WireframeLoad.LoadWireframe` (`self.WireframeLoad`))
      (`self.K2_DestroyActor`))
    (:`then_5`
      (bind _asbp_game_instance (cast `/Game/Blueprints/BP_GameInstance` (`GameplayStatics.GetGameInstance`)))
      (`/Game/Blueprints/BP_GameInstance.PlayInGameMusic` _asbp_game_instance))))

(fn `CreateSetMaterialInstance`
  (bind _mesh (`self.Mesh`))
  (bind _mesh_2 (`self.Mesh`))
  (bind _returnvalue (`PrimitiveComponent.GetMaterial` _mesh 0))
  (bind _returnvalue_2 (`PrimitiveComponent.GetMaterial` _mesh_2 1))
  (`/Engine/EditorBlueprintResources/StandardMacros.IsValid` _returnvalue
    (:`Is Valid`
      (bind _returnvalue_3 (`KismetMaterialLibrary.CreateDynamicMaterialInstance` _returnvalue))
      (set `self.ModuleMaterialInstance` _returnvalue_3)
      (`PrimitiveComponent.SetMaterial` _mesh 0 null)
      (`/Engine/EditorBlueprintResources/StandardMacros.IsValid` _returnvalue_2
        (:`Is Valid`
          (bind _returnvalue_4 (`KismetMaterialLibrary.CreateDynamicMaterialInstance` _returnvalue_2))
          (set `self.ScreenMaterialInstance` _returnvalue_4)
          (`PrimitiveComponent.SetMaterial` _mesh_2 1 null))))))

(fn `UserConstructionScript`
  (`parent.UserConstructionScript`))