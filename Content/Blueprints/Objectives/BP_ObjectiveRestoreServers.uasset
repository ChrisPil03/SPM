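; BP_ObjectiveRestoreServers is the restore-servers objective Blueprint, which shows on-screen messages when the objective starts or completes.
; BeginPlay creates a WBP_ObjectiveMessage widget for player 0 and caches it for reuse.
; The description and completed events set "Started" or "Completed", briefly add the widget to the viewport, then remove it after a delay.
; A stop event removes it immediately; no server-restoration logic is implemented here.
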(event `self.DisplayObjectiveDescription`
  (bind _objectivemessageinstance (`self.ObjectiveMessageInstance`))
  (bind _objectivemessageinstance_2 (`self.ObjectiveMessageInstance`))
  ; Display Objective Message On Screen
  (if (`KismetSystemLibrary.IsValid` _objectivemessageinstance_2)
    (`/Game/Blueprints/Widgets/WBP_ObjectiveMessage.SetObjectiveMessageText` _objectivemessageinstance_2 "Started")
    (`UserWidget.AddToViewport` _objectivemessageinstance 0)
    (`KismetSystemLibrary.Delay` 2.0)
    (`Widget.RemoveFromParent` _objectivemessageinstance)
    (else
      (`KismetSystemLibrary.PrintString` "Object Message Instance not valid"))))

(event `self.DisplayObjectiveCompleted`
  (bind _objectivemessageinstance (`self.ObjectiveMessageInstance`))
  (bind _objectivemessageinstance_2 (`self.ObjectiveMessageInstance`))
  ; Display Objective Completed
  (if (`KismetSystemLibrary.IsValid` _objectivemessageinstance_2)
    (`/Game/Blueprints/Widgets/WBP_ObjectiveMessage.SetObjectiveMessageText` _objectivemessageinstance_2 "Completed")
    (`UserWidget.AddToViewport` _objectivemessageinstance 0)
    (`KismetSystemLibrary.Delay` 2.0)
    (`Widget.RemoveFromParent` _objectivemessageinstance)
    (else
      (`KismetSystemLibrary.PrintString` "Object Message Instance not valid"))))

(event `self.StopDisplayObjectiveDescription`
  (bind _objectivemessageinstance (`self.ObjectiveMessageInstance`))
  ; Remove Objective Message from Viewport
  (if (`KismetSystemLibrary.IsValid` _objectivemessageinstance)
    (`Widget.RemoveFromParent` _objectivemessageinstance)
    (else
      (`KismetSystemLibrary.PrintString` "Object Message Instance not valid"))))

(event `self.ReceiveBeginPlay`
  ; Begin Play
  (bind _returnvalue (`|CreateWidget` "/Game/Blueprints/Widgets/WBP_ObjectiveMessage.WBP_ObjectiveMessage_C" (`GameplayStatics.GetPlayerController` 0)))
  (set `self.ObjectiveMessageInstance` _returnvalue))

(fn `UserConstructionScript`)