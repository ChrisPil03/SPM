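; BP_TimedTaskInteractable is a timed-task objective interactable that gives visual feedback through an animated lever.
; At BeginPlay it creates a dynamic material instance for slot 1 of Mesh and binds to the interact and activated delegates.
; Interacting clears the material's "Is Paused" parameter and plays the pull animation, while activation sets it and plays the reset animation.
; Screen material logic is present but disconnected.
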(event `self.ReceiveBeginPlay`
  (`self.CreateSetMaterialInstances`)
  (add `self.InteractDelegate` (delegate `OnInteractEvent`))
  (add `self.OnActivated` (delegate `OnActivatedEvent`)))

(event `OnActivatedEvent`
  (`MaterialInstanceDynamic.SetScalarParameterValue` (`self.LeverMaterialInstance`) "Is Paused" 1.0)
  (`SkeletalMeshComponent.PlayAnimation` (`self.Lever`) (`self.ResetLeverAnimation`) false))

(event `OnInteractEvent` :!signature `self.InteractDelegate`
  (params (Object :type "InteractableObject Object Reference"))
  (`MaterialInstanceDynamic.SetScalarParameterValue` (`self.LeverMaterialInstance`) "Is Paused" 0.0)
  (`SkeletalMeshComponent.PlayAnimation` (`self.Lever`) (`self.PullLeverAnimation`) false))

(fn `CreateSetMaterialInstances`
  (bind _mesh (`self.Mesh`))
  (bind _returnvalue (`PrimitiveComponent.GetMaterial` _mesh 1))
  (`/Engine/EditorBlueprintResources/StandardMacros.IsValid` _returnvalue
    (:`Is Valid`
      (bind _returnvalue_2 (`KismetMaterialLibrary.CreateDynamicMaterialInstance` _returnvalue))
      (bind _output_get (set `self.LeverMaterialInstance` _returnvalue_2))
      (`PrimitiveComponent.SetMaterial` _mesh 1 _output_get))))

(fn `UserConstructionScript`)