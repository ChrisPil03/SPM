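; MyGun is a gun Blueprint that routes firing and reloading through the Gameplay Ability System.
; Fire and Reload activate GA_FireWeapon and GA_Reload by class on the gun's ability system component.
; StartFire fires immediately and, for automatic guns, starts a looping timer by function name that StopFire clears.
; On BeginPlay it binds to the WeaponAttributeSet's ammo-changed event to update the ammo widget's magazine text.
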(event `self.SetAmmoCountText`
  (params (Ammo :type "Float (single-precision)"))
  (bind _ammowidget (`self.AmmoWidget`))
  (`/Engine/EditorBlueprintResources/StandardMacros.IsValid` _ammowidget
    (:`Is Valid`
      (`/Game/Blueprints/Widgets/WBP_Ammunition.SetAmmoInMagText` _ammowidget (`KismetMathLibrary.FTrunc` Ammo)))))

(event `self.ReceiveBeginPlay`
  (bind _returnvalue (`AbilitySystemComponent.GetAttributeSet` (`AbilitySystemBlueprintLibrary.GetAbilitySystemComponent` null) "/Script/CoolGang.WeaponAttributeSet"))
  (add `WeaponAttributeSet.OnAmmoChanged` _returnvalue (delegate `self.SetAmmoCountText`)))

(event `self.StartFire`
  (if (`self.bIsAutomatic`)
    (`self.Fire`)
    (bind _returnvalue (`KismetSystemLibrary.K2_SetTimer` null (`self.Fire Function Name`) (`self.TimeBetweenShots`) true))
    (else
      (`self.Fire`))))

(event `self.StopFire`
  (`KismetSystemLibrary.K2_ClearAndInvalidateTimerHandle` (stale `self.StartFire` _returnvalue)))

(event `self.Fire`
  (`AbilitySystemComponent.TryActivateAbilityByClass` (`AbilitySystemBlueprintLibrary.GetAbilitySystemComponent` null) "/Game/Blueprints/GAS/GA_FireWeapon.GA_FireWeapon_C" true))

(event `self.Reload`
  (`AbilitySystemComponent.TryActivateAbilityByClass` (`AbilitySystemBlueprintLibrary.GetAbilitySystemComponent` null) "/Game/Blueprints/GAS/GA_Reload.GA_Reload_C" true))

(fn `UserConstructionScript`)