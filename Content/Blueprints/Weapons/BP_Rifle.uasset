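; Rifle weapon Blueprint that extends its parent weapon with a laser beam fire mode during the ultimate.
; Ultimate start and end delegates swap the fire GameplayEffect between normal and laser.
; While tagged Status.OnUltimate, firing starts the BP_Beam child actor, then a short timer triggers parent fire and laser audio.
; Stopping fire or ending the ultimate clears that timer and ends beam and audio; unequipping mid-ultimate cancels the beam instead of calling parent.
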(event `self.ReceiveBeginPlay`
  (`parent.ReceiveBeginPlay`)
  (set `self.WeaponIconImage` (`/Game/Blueprints/Widgets/WBP_WeaponIconRifle.BackgroundImage` (`/Game/Blueprints/Widgets/WBP_CenterPanel.WBP_WeaponIconRifle` (`self.Widget`))))
  (add `self.OnUltimateStartDelegate` (delegate `CustomEvent`))
  (add `self.OnUltimateEndDelegate` (delegate `CustomEvent_1`))
  (set `self.NewSkin` "/Game/Assets/Materials/Weapons/Rifle/Secret/M_Rifle_Secret.M_Rifle_Secret"))

(event `CustomEvent`
  (set `self.GameplayEffectToActivateWhenFire` "/Game/Blueprints/GAS/Weapons/Effects/GE_Fire_Laser.GE_Fire_Laser_C"))

(event `CustomEvent_1`
  (set `self.GameplayEffectToActivateWhenFire` "/Game/Blueprints/GAS/Weapons/Effects/GE_Fire.GE_Fire_C")
  (bind _asbp_beam (cast `/Game/Blueprints/VFX_BP/BP_Beam` (`ChildActorComponent.ChildActor` (`self.Beam`))))
  (`/Game/Blueprints/VFX_BP/BP_Beam.EndBeam` _asbp_beam)
  (`KismetSystemLibrary.K2_ClearAndInvalidateTimerHandle` (stale `self.StartFire` _returnvalue))
  (`|ExecutionSequence`
    (:`then_0`
      (if (`self.bIsBeaming`)
        (bind _asbp_beam_2 (cast `/Game/Blueprints/VFX_BP/BP_Beam` (`ChildActorComponent.ChildActor` (`self.Beam`))))
        (`/Game/Blueprints/VFX_BP/BP_Beam.EndBeam` _asbp_beam_2)))
    (:`then_1`
      (if (`self.bIsFiring`)
        (`AudioParameterControllerInterface.SetTriggerParameter` (`self.LaserAudio`) "Stop")))))

(event `self.OnUnequipped`
  (if (`GameplayTagAssetInterface.HasMatchingGameplayTag` (`self.AbilitySystemComponent`) (struct :`TagName` "Status.OnUltimate"))
    (`KismetSystemLibrary.PrintString` "cannel beam")
    (bind _asbp_beam (cast `/Game/Blueprints/VFX_BP/BP_Beam` (`ChildActorComponent.ChildActor` (`self.Beam`))))
    (`/Game/Blueprints/VFX_BP/BP_Beam.Cancel` _asbp_beam)
    (else
      (`parent.OnUnequipped`))))

(event `self.StartFire`
  (if (`GameplayTagAssetInterface.HasMatchingGameplayTag` (`self.AbilitySystemComponent`) (struct :`TagName` "Status.OnUltimate"))
    (bind _asbp_beam (cast `/Game/Blueprints/VFX_BP/BP_Beam` (`ChildActorComponent.ChildActor` (`self.Beam`))))
    (`/Game/Blueprints/VFX_BP/BP_Beam.StartBeam` _asbp_beam)
    (set `self.bIsBeaming` true)
    (bind _returnvalue (`KismetSystemLibrary.K2_SetTimerDelegate` (delegate `UltimateFire`) 0.9))
    (else
      (`parent.StartFire`))))

(event `UltimateFire`
  (bind _laseraudio (`self.LaserAudio`))
  (`parent.StartFire`)
  (`AudioComponent.Play` _laseraudio 0.0)
  (`AudioParameterControllerInterface.SetTriggerParameter` _laseraudio "Play"))

(event `self.StopFire`
  (if (`GameplayTagAssetInterface.HasMatchingGameplayTag` (`self.AbilitySystemComponent`) (struct :`TagName` "Status.OnUltimate"))
    (`KismetSystemLibrary.K2_ClearAndInvalidateTimerHandle` (stale `self.StartFire` _returnvalue))
    (`|ExecutionSequence`
      (:`then_0`
        (if (`self.bIsBeaming`)
          (bind _asbp_beam (cast `/Game/Blueprints/VFX_BP/BP_Beam` (`ChildActorComponent.ChildActor` (`self.Beam`))))
          (`/Game/Blueprints/VFX_BP/BP_Beam.EndBeam` _asbp_beam)))
      (:`then_1`
        (if (`self.bIsFiring`)
          (`AudioParameterControllerInterface.SetTriggerParameter` (`self.LaserAudio`) "Stop")))
      (:`then_2`
        (`parent.StopFire`)))
    (else
      (`parent.StopFire`))))

(event `self.ActivateAbility`
  (`self.StopFire`)
  (`parent.ActivateAbility`))

(fn `UserConstructionScript`
  (`parent.UserConstructionScript`))