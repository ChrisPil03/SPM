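; BP_Pistol is the handgun weapon Blueprint, which changes its fire ability and bullet sound while an ultimate is active.
; On BeginPlay it takes its icon image from the handgun icon widget and binds to the ultimate start and end delegates.
; Ultimate start switches to GA_Fire_Chaining, granting it on every start, and the ultimate sound.
; Ultimate end restores GA_FireWeapon and the normal sound without removing the granted ability.
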(event `self.ReceiveBeginPlay`
  (`parent.ReceiveBeginPlay`)
  (set `self.WeaponIconImage` (`/Game/Blueprints/Widgets/WBP_WeaponIconHandgun.BackgroundImage` (`/Game/Blueprints/Widgets/WBP_CenterPanel.WBP_WeaponIconHandgun` (`self.Widget`))))
  (add `self.OnUltimateStartDelegate` (delegate `CustomEvent`))
  (add `self.OnUltimateEndDelegate` (delegate `CustomEvent_1`)))

(event `CustomEvent_1`
  (bind _normalbulletsound (`self.NormalBulletSound`))
  (set `self.FireAbilityClass` "/Game/Blueprints/GAS/Weapons/Abilities/GA_FireWeapon.GA_FireWeapon_C")
  (`/Engine/EditorBlueprintResources/StandardMacros.IsValid` _normalbulletsound
    (:`Is Valid`
      (set `self.BulletSound` _normalbulletsound))))

(event `CustomEvent`
  (bind _ultimatebulletsound (`self.UltimateBulletSound`))
  (set `self.FireAbilityClass` "/Game/Blueprints/GAS/Weapons/Abilities/GA_Fire_Chaining.GA_Fire_Chaining_C")
  (`AbilitySystemComponent.K2_GiveAbility` (`self.AbilitySystemComponent`) "/Game/Blueprints/GAS/Weapons/Abilities/GA_Fire_Chaining.GA_Fire_Chaining_C" 0 -1)
  (`/Engine/EditorBlueprintResources/StandardMacros.IsValid` _ultimatebulletsound
    (:`Is Valid`
      (set `self.BulletSound` _ultimatebulletsound))))

(fn `UserConstructionScript`
  (`parent.UserConstructionScript`))