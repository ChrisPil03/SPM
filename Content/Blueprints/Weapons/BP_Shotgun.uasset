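; Shotgun weapon Blueprint that extends a parent weapon with its own icon, skin and ultimate-dependent impact effect.
; On BeginPlay, after the parent logic, it sets the icon from the shotgun icon widget's background image and assigns the M_ShotgunOrca skin.
; It binds to the ultimate start and end delegates to switch the impact effect between ultimate and normal versions, when those are valid.
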(event `self.ReceiveBeginPlay`
  (`parent.ReceiveBeginPlay`)
  (set `self.WeaponIconImage` (`/Game/Blueprints/Widgets/WBP_WeaponIconShotgun.BackgroundImage` (`/Game/Blueprints/Widgets/WBP_CenterPanel.WBP_WeaponIconShotgun` (`self.Widget`))))
  (add `self.OnUltimateStartDelegate` (delegate `CustomEvent`))
  (add `self.OnUltimateEndDelegate` (delegate `CustomEvent_1`))
  (set `self.NewSkin` "/Game/Assets/Materials/Weapons/Shotgun/M_ShotgunOrca.M_ShotgunOrca"))

(event `CustomEvent`
  (bind _ultimateimpacteffect (`self.UltimateImpactEffect`))
  (`/Engine/EditorBlueprintResources/StandardMacros.IsValid` _ultimateimpacteffect
    (:`Is Valid`
      (set `self.ImpactEffect` _ultimateimpacteffect))))

(event `CustomEvent_1`
  (bind _normalimpacteffect (`self.NormalImpactEffect`))
  (`/Engine/EditorBlueprintResources/StandardMacros.IsValid` _normalimpacteffect
    (:`Is Valid`
      (set `self.ImpactEffect` _normalimpacteffect))))

(fn `UserConstructionScript`
  (`parent.UserConstructionScript`))