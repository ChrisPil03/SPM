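; Weapon Blueprint that drives firing, reloading and an ultimate through Gameplay Ability System abilities.
; StartFire is gated by a shot-interval timer, with a looping timer repeating Fire for automatic weapons until StopFire.
; Ammo and magazine-size delegates update the widget, and low ammo triggers an automatic reload.
; A Material Parameter Collection scalar drives the ammo ring, set from the ammo ratio or animated by the reload timeline.
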(event `CustomEvent` :!signature `self.OnMagazineSizeChangedDelegate`
  (params (MagazineSize :type "Float (single-precision)"))
  (bind _widget (`self.Widget`))
  (`/Engine/EditorBlueprintResources/StandardMacros.IsValid` _widget
    (:`Is Valid`
      (if (not (`self.bHidden`))
        (`/Game/Blueprints/Widgets/WBP_CenterPanel.SetMagazineSizeText` _widget (`KismetMathLibrary.Conv_IntToDouble` (`KismetMathLibrary.FTrunc` MagazineSize)))))))

(event `self.ReceiveBeginPlay`
  (add `self.OnAmmoCountChangedDelegate` (delegate `self.SetAmmoCountText`))
  (add `self.OnMagazineSizeChangedDelegate` (delegate `CustomEvent`)))

(event `self.SetAmmoCountText`
  (params (Ammo :type "Float (single-precision)"))
  (bind _returnvalue (`KismetMathLibrary.FTrunc` Ammo))
  (bind _widget (`self.Widget`))
  (`|ExecutionSequence`
    (:`then_0`
      (`/Engine/EditorBlueprintResources/StandardMacros.IsValid` _widget
        (:`Is Valid`
          (if (not (`self.bHidden`))
            (`/Game/Blueprints/Widgets/WBP_CenterPanel.SetAmmoInMagText` _widget _returnvalue)
            (`self.UpdateAmmoRing` Ammo (stale `CustomEvent` MagazineSize))))))
    (:`then_1`
      (if (< _returnvalue 1.0)
        (`self.Reload`)))))

(event `self.StartFire`
  (bind _timebetweenshots (`self.TimeBetweenShots`))
  (if (`self.bCanFire`)
    (if (`self.bIsAutomatic`)
      (`self.Fire`)
      (bind _returnvalue (`KismetSystemLibrary.K2_SetTimer` null (`self.Fire Function Name`) _timebetweenshots true))
      (`KismetSystemLibrary.K2_SetTimerDelegate` (delegate `OnFireFinished`) _timebetweenshots)
      (set `self.bCanFire` false)
      (else
        (`self.Fire`)
        (`KismetSystemLibrary.K2_SetTimerDelegate` (delegate `OnFireFinished`) _timebetweenshots)
        (set `self.bCanFire` false)))))

(event `self.StopFire`
  (`KismetSystemLibrary.K2_ClearAndInvalidateTimerHandle` (stale `self.StartFire` _returnvalue)))

(event `OnFireFinished`
  (set `self.bCanFire` true))

(event `self.Fire`
  (`AbilitySystemComponent.TryActivateAbilityByClass` (`AbilitySystemBlueprintLibrary.GetAbilitySystemComponent` null) "/Game/Blueprints/GAS/Weapons/Abilities/GA_FireWeapon.GA_FireWeapon_C" true))

(event `self.Reload`
  (`AbilitySystemComponent.TryActivateAbilityByClass` (`AbilitySystemBlueprintLibrary.GetAbilitySystemComponent` null) "/Game/Blueprints/GAS/Weapons/Abilities/GA_Reload.GA_Reload_C" true)
  (bind (_direction _reloadtimeline) (`Timeline|ReloadMaterialTimeline` :!via `PlayFromStart`)
    (:`Update`
      (`KismetMaterialLibrary.SetScalarParameterValue` (`self.RingMPC`) (`self.RingParamName`) _reloadtimeline))))

(event `self.ActivateAbility`
  (bind _returnvalue (`AbilitySystemBlueprintLibrary.GetAbilitySystemComponent` null))
  (bind _returnvalue_2 (`AbilitySystemComponent.TryActivateAbilityByClass` _returnvalue "/Game/Blueprints/GAS/Weapons/Abilities/GA_Ultimate.GA_Ultimate_C" true))
  (if _returnvalue_2
    (`KismetSystemLibrary.PrintString` "activate ultimate")
    (`AbilitySystemComponent.ClearAbility` _returnvalue (`self.GunAbility`))))

(fn `UpdateAmmoRing`
  (params (CurrentAmmo :type "Float (double-precision)") (MaxAmmo :type "Float (double-precision)"))
  (bind _output_get (set `self.CurrentAmmoFloat` (/ CurrentAmmo MaxAmmo)))
  (`KismetMaterialLibrary.SetScalarParameterValue` (`self.RingMPC`) (`self.RingParamName`) _output_get))

(fn `UserConstructionScript`)