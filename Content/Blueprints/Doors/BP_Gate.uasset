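; BP_Gate is a gate actor that opens and closes through its Open and Close events.
; Each event plays its animation sequence once on the skeletal mesh, toggles the doors' box collision and updates the IsOpen flag.
; Collision switches off as soon as the opening animation starts and back on as soon as closing starts, without waiting for either animation to finish.
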(event `self.Open`
  (`SkeletalMeshComponent.PlayAnimation` (`self.SkeletalMesh`) (`self.OpenAnimationSequence`) false)
  (`PrimitiveComponent.SetCollisionEnabled` (`self.DoorsBoxCollision`) "NoCollision")
  (set `self.bIsOpen` true))

(event `self.Close`
  (`SkeletalMeshComponent.PlayAnimation` (`self.SkeletalMesh`) (`self.CloseAnimationSequence`) false)
  (`PrimitiveComponent.SetCollisionEnabled` (`self.DoorsBoxCollision`) "QueryAndPhysics")
  (set `self.bIsOpen` false))

(fn `UserConstructionScript`)