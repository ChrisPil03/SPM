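; BP_LoadNewLevel is an overlap trigger that moves the player from the current streamed level to the next one.
; When BP_PlayerCharacter overlaps it, it starts a non-blocking load of LevelToLoad and immediately moves the player to the Capsule component's location.
; It then calls DestroyDownloadZone on every BP_ObjectiveDownloadStation.
; CurrentLevel's unload sits inside that loop, so it repeats per station and never runs without one.
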(event `self.ReceiveActorBeginOverlap`
  (params (OtherActor :type "Actor Object Reference"))
  (bind _asbp_player_character (cast `/Game/Blueprints/BP_PlayerCharacter` OtherActor))
  (`GameplayStatics.LoadStreamLevel` (`self.LevelToLoad`) true)
  (`self.K2_SetActorLocation` _asbp_player_character (`SceneComponent.K2_GetComponentLocation` (`self.Capsule`)) false false)
  (bind _outactors (`GameplayStatics.GetAllActorsOfClass` "/Game/Blueprints/Objectives/BP_ObjectiveDownloadStation.BP_ObjectiveDownloadStation_C"))
  (for _array_element _outactors
    (`ObjectiveDownloadStation.DestroyDownloadZone` _array_element)
    (`GameplayStatics.UnloadStreamLevel` (`self.CurrentLevel`))))

(fn `UserConstructionScript`)