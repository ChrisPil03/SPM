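; Debug interactable actor that hands out the GA_Debug gameplay ability for testing.
; On BeginPlay it grants the ability to its own ability system component.
; When a BP_PlayerCharacter interacts, it grants the ability to the equipped gun's ability system and stores the returned handle as that weapon's GunAbility.
; A leftover node for spawning a BP_PickupBase is unconnected and never runs.
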(event `self.ReceiveBeginPlay`
  (`AbilitySystemComponent.K2_GiveAbility` (`self.AbilitySystem`) "/Game/Blueprints/GAS/GA_Debug.GA_Debug_C" 0 -1))

(event `self.Interact`
  (params (Interactor :type "Actor Object Reference"))
  (bind _asbp_player_character (cast `/Game/Blueprints/BP_PlayerCharacter` Interactor))
  (bind _returnvalue (`PlayerCharacter.GetEquippedGun` _asbp_player_character))
  (bind _returnvalue_2 (`AbilitySystemComponent.K2_GiveAbility` (`AbilitySystemBlueprintLibrary.GetAbilitySystemComponent` _returnvalue) "/Game/Blueprints/GAS/GA_Debug.GA_Debug_C" 0 -1))
  (bind _asbp_weapon (cast `/Game/Blueprints/Weapons/BP_Weapon` _returnvalue))
  (set `/Game/Blueprints/Weapons/BP_Weapon.GunAbility` _returnvalue_2 _asbp_weapon))

(fn `UserConstructionScript`)